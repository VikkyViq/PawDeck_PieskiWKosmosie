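; D_Ciastko_BP is a dialogue trigger actor that shows "Ciastko" (cookie) dialogue widgets when the player interacts near it.
; A Box overlap with the 3Piesek actor opens a gate for the Interaction input and closes it on exit.
; The first interaction adds D_Ciastko_2 to the viewport and sets DidPlayAlready, so later presses show D_Ciastko_3 instead.
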(event `self.ReceiveBeginPlay`
  (`self.EnableInput` (`GameplayStatics.GetPlayerController` 0)))

(event `InputAction|Interaction`
  (params (Key :type "Key Structure"))
  (:`Pressed`
    (`/Engine/EditorBlueprintResources/StandardMacros.Gate` true :!label _label
      (:`Exit`
        (if (`self.DidPlayAlready?`)
          (bind _returnvalue (`|CreateWidget` "/Game/Dialogi/Ciastko/D_Ciastko_3.D_Ciastko_3_C"))
          (`UserWidget.AddToViewport` _returnvalue 0)
          (else
            (bind _returnvalue_2 (`|CreateWidget` "/Game/Dialogi/Ciastko/D_Ciastko_2.D_Ciastko_2_C"))
            (`UserWidget.AddToViewport` _returnvalue_2 0)
            (set `self.DidPlayAlready?` true)))))))

(event `self.Box.OnComponentBeginOverlap`
  (params (OverlappedComponent :type "PrimitiveComponent Object Reference") (OtherActor :type "Actor Object Reference") (OtherComp :type "PrimitiveComponent Object Reference") (OtherBodyIndex :type Integer) (bFromSweep :type Boolean) (SweepResult :type "HitResult Structure (by ref)"))
  (`self.EnableInput` (`GameplayStatics.GetPlayerController` 0))
  (cast `/Game/ThirdPersonBP/Blueprints/3Piesek` OtherActor)
  (goto _label :!via `Open`))

(event `self.Box.OnComponentEndOverlap`
  (params (OverlappedComponent :type "PrimitiveComponent Object Reference") (OtherActor :type "Actor Object Reference") (OtherComp :type "PrimitiveComponent Object Reference") (OtherBodyIndex :type Integer))
  (cast `/Game/ThirdPersonBP/Blueprints/3Piesek` OtherActor)
  (goto _label :!via `Close`))

(fn `UserConstructionScript`)